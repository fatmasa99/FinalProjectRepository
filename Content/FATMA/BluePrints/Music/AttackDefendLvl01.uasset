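; Music trigger Blueprint that plays the AttackDefendLvl01 audio event, attached, when MainCharacter_BP overlaps its Box.
; Tick accumulates and prints a timer, resetting it to zero once it reaches ten seconds.
; The overlap prints the character's name and plays the event only if the timer is at least ten, a state Tick clears in the same update it occurs.
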(event OnComponentBeginOverlap(Box)
  (params (OverlappedComponent :type Primitive%20Component%20Object%20Reference) (OtherActor :type Actor%20Object%20Reference) (OtherComp :type Primitive%20Component%20Object%20Reference) (OtherBodyIndex :type Integer) (bFromSweep :type Boolean) (SweepResult :type Hit%20Result%20Structure%20%28by%20ref%29))
  (Utilities|Casting|CastToMainCharacter_BP OtherActor)
  (Development|PrintString (Utilities|GetDisplayName OtherActor) true true "(R=1.000000,G=0.848204,B=0.000000,A=1.000000)")
  (if (not (< (Variables|Default|GetTimer) 1e+01))
    (Class|FMODBlueprintStatics|PlayEventAttached "/Game/FMOD/Events/MusicFirstLevel/AttackDefendLvl01.AttackDefendLvl01" 0 "None" "0, 0, 0" "KeepRelativeOffset")))

(event EventBeginPlay)

(event Collision|EventActorBeginOverlap
  (params (OtherActor :type Actor%20Object%20Reference)))

(event EventTick
  (params (DeltaSeconds :type Float%20%28single-precision%29))
  (bind _output_get (Variables|Default|SetTimer (+ DeltaSeconds (Variables|Default|GetTimer))))
  (Development|PrintString (Utilities|String|ToString(Float) (Variables|Default|GetTimer)) true true "(R=1.000000,G=0.000000,B=0.098634,A=1.000000)")
  (if (>= _output_get 1e+01)
    (Variables|Default|SetTimer 0.0)))

(fn ConstructionScript)