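; PaperZD animation notify that runs a hit check at the "Defend01" socket for a defend animation.
; With a valid owning instance, it box-overlaps Pawns at the socket, ignoring the owner, and launches any HitDetectionTestCharacter straight up.
; Without one, presumably in editor preview, it draws a brief debug box at the socket, slightly larger than the actual overlap box.
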(event EventOnReceiveNotify
  (params (OwningInstance :type Paper%20ZD%20Anim%20Instance%20Object%20Reference))
  (bind _sequencerendercomponent (Variables|Default|GetSequenceRenderComponent))
  (bind _returnvalue (Transformation|GetSocketLocation _sequencerendercomponent "Defend01"))
  (Utilities|IsValid OwningInstance
    (:Is%20Valid
      (bind _outactors (Collision|BoxOverlapActors _returnvalue "25.000000,25.000000,25.000000" (Utilities|Array|MakeArray "ObjectTypeQuery3") 0 (Utilities|Array|MakeArray (Class|PaperZDAnimInstance|GetOwningActor OwningInstance)) :!class /Script/Engine.KismetSystemLibrary))
      (for _array_element _outactors
        (bind _ashit_detection_test_character (Utilities|Casting|CastToHitDetectionTestCharacter _array_element))
        (Character|LaunchCharacter _ashit_detection_test_character (* (Math|Vector|VectorUp) 5e+02) false false)))
    (:Is%20Not%20Valid
      (Rendering|Debug|DrawDebugBox _returnvalue "30.000000,30.000000,30.000000" "(R=1.000000,G=0.000000,B=0.465934,A=1.000000)" "0, 0, 0" 1.0 1.0))))