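; HitDetectionTestCharacter is a test character for hit detection that can both deal and receive damage.
; Overlapping its CauseDanageTest component calls TakeDamage on a MainCharacter_BP and prints that character's Life.
; Any damage it receives destroys it immediately, with no health check.
; A SpawnDust function spawns Land_smoke at the sprite's location and rotation, but nothing in this graph calls it.
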(event OnComponentBeginOverlap(CauseDanageTest)
  (params (OverlappedComponent :type Primitive%20Component%20Object%20Reference) (OtherActor :type Actor%20Object%20Reference) (OtherComp :type Primitive%20Component%20Object%20Reference) (OtherBodyIndex :type Integer) (bFromSweep :type Boolean) (SweepResult :type Hit%20Result%20Structure%20%28by%20ref%29))
  (bind _asmain_character_bp (Utilities|Casting|CastToMainCharacter_BP OtherActor))
  (Default|TakeDamage _asmain_character_bp)
  (Development|PrintString (Utilities|String|ToString(Float) (Variables|/Game/FATMA/BluePrints/MainCharacter/MainCharacter_BP.MainCharacter_BP_C|GetLife _asmain_character_bp))))

(event Game|Damage|EventAnyDamage
  (params (Damage :type Float%20%28single-precision%29) (DamageType :type Damage%20Type%20Object%20Reference) (InstigatedBy :type Controller%20Object%20Reference) (DamageCauser :type Actor%20Object%20Reference))
  (Actor|DestroyActor))

(fn ConstructionScript)

(fn SpawnDust
  (bind _sprite (Variables|Default|GetSprite))
  (bind _returnvalue (Transformation|GetWorldTransform _sprite))
  (Game|SpawnActorfromClass "/Game/FATMA/BluePrints/Effects/Land_smoke.Land_smoke_C" (Math|Transform|MakeTransform (.location _returnvalue) (.rotation _returnvalue) "1.000000,1.000000,1.000000") "AlwaysSpawn" 0 0))