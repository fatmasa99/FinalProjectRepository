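; PaperZD animation notify that performs sword hit detection for the first attack.
; When received, it runs a box overlap for pawns at the SwordAttack01 socket, ignoring the owning actor, and applies fixed damage to each actor found, with debug prints.
; Without a valid owning instance, it instead draws a debug box of the same extent at that socket, which allows visualizing the hit area.
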(event EventOnReceiveNotify
  (params (OwningInstance :type Paper%20ZD%20Anim%20Instance%20Object%20Reference))
  (bind _sequencerendercomponent (Variables|Default|GetSequenceRenderComponent))
  (bind _returnvalue (Transformation|GetSocketLocation _sequencerendercomponent "SwordAttack01"))
  (Utilities|IsValid OwningInstance
    (:Is%20Valid
      (bind _outactors (Collision|BoxOverlapActors _returnvalue (Variables|Default|GetExtent) (Utilities|Array|MakeArray "ObjectTypeQuery3") 0 (Utilities|Array|MakeArray (Class|PaperZDAnimInstance|GetOwningActor OwningInstance)) :!class /Script/Engine.KismetSystemLibrary))
      (for _array_element _outactors
        (Development|PrintString (Utilities|GetDisplayName _array_element))
        (Game|Damage|ApplyDamage _array_element 1e+01 0 0))
      (Development|PrintString "NoMoreActorsFound"))
    (:Is%20Not%20Valid
      (Rendering|Debug|DrawDebugBox _returnvalue (Variables|Default|GetExtent) "(R=1.000000,G=0.069179,B=0.561482,A=1.000000)" "0, 0, 0" 1.0 1.0))))