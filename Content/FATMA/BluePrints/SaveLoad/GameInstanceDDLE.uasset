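; Game instance Blueprint with Save and Load events for the player character's position, using a SaveGameDDLE object and a single save slot.
; Save records the location in PlayerPos, creating the save object if none is valid, and writes to the slot only in that creation branch.
; Load checks that the slot exists, casts and caches the loaded object, then moves the player character to its stored PlayerPos.
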(event Custom|Save
  (bind _returnvalue (Game|GetPlayerCharacter 0))
  (bind _returnvalue_2 (Transformation|GetActorLocation _returnvalue))
  (Utilities|IsValid (Variables|Default|GetSaveGame)
    (:Is%20Valid
      (Variables|Default|SetPlayerPos _returnvalue_2))
    (:Is%20Not%20Valid
      (bind _returnvalue_3 (SaveGame|CreateSaveGameObject "/Game/FATMA/BluePrints/SaveLoad/SaveGameDDLE.SaveGameDDLE_C"))
      (Variables|Default|SetSaveGame _returnvalue_3)
      (Variables|Default|SetPlayerPos _returnvalue_2)
      (SaveGame|SaveGametoSlot (Variables|Default|GetSaveGame) "Slot0"))))

(event Custom|Load
  (bind _returnvalue (SaveGame|DoesSaveGameExist "Slot0"))
  (if _returnvalue
    (bind _returnvalue_2 (SaveGame|LoadGamefromSlot "Slot0"))
    (bind _assave_game_ddle (Utilities|Casting|CastToSaveGameDDLE _returnvalue_2))
    (bind _output_get (Variables|Default|SetSaveGame _assave_game_ddle))
    (Transformation|SetActorLocation (Game|GetPlayerCharacter 0) (Variables|/Game/FATMA/BluePrints/SaveLoad/SaveGameDDLE.SaveGameDDLE_C|GetPlayerPos _output_get) false false)))