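; Fatma enemy for a sprite-based side-scroller that walks along X and reacts to the player.
; Each Tick a sphere trace detects the player: if found, an eye-level line trace sets Attack and movement input follows player X location and velocity.
; Otherwise it walks in its facing direction, reversing on capsule hits.
; Ledge traces, Patrol and Movement are unfinished helpers outside the Tick flow, and traces draw debug shapes.
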(event OnComponentHit(CapsuleComponent)
  (params (HitComponent :type Primitive%20Component%20Object%20Reference) (OtherActor :type Actor%20Object%20Reference) (OtherComp :type Primitive%20Component%20Object%20Reference) (NormalImpulse :type Vector :default "0, 0, 0") (Hit :type Hit%20Result%20Structure%20%28by%20ref%29))
  (bind _output_get (Variables|Default|SetisMovingRight? (not (Variables|Default|GetisMovingRight?))))
  (Development|PrintString (Utilities|String|ToString(Boolean) _output_get) true true "(R=0.657705,G=0.000000,B=1.000000,A=1.000000)"))

(event Custom|Direction
  (Transformation|SetRelativeRotation (Variables|Default|GetSprite) (Math|Rotator|MakeRotator 0.0 0.0 (Math|Float|SelectFloat 0.0 1.8e+02 (Variables|Default|GetisMovingRight?))) false false)
  (Pawn|Input|AddMovementInput (Math|Vector|SelectVector "1.000000,0.000000,0.000000" "-1.000000,0.000000,0.000000" (Variables|Default|GetisMovingRight?)) 1.0 false))

(event Custom|EnemyStart
  (bind _detected (CallFunction|SingleSphereCheck))
  (bind _output_get (Variables|Default|SetChDetected _detected))
  (if _output_get
    (bind _attack (CallFunction|CheckVision (Variables|Default|GetPlayerRef)))
    (Variables|Default|SetAttack _attack)
    (CallFunction|FollowCharacter)
    (else
      (Variables|Default|SetAttack false)
      (CallFunction|Direction))))

(event Custom|FollowCharacter
  (bind _playerref (Variables|Default|GetPlayerRef))
  (if (Variables|Default|GetChDetected)
    (Pawn|Input|AddMovementInput (Math|Vector|MakeVector (.x (Transformation|GetWorldLocation (Variables|/Script/Engine.Character|GetCapsuleComponent _playerref))) 0.0 0.0) (.x (Transformation|GetVelocity _playerref)) false)))

(event EventBeginPlay
  (Utilities|FlowControl|Sequence
    (:then_0
      (bind _asmain_character_bp (Utilities|Casting|CastToMainCharacter_BP (Game|Player|GetPlayerPawn 0)))
      (Variables|Default|SetPlayerRef _asmain_character_bp))
    (:then_1
      (Variables|Default|SetDirection (Transformation|GetVelocity)))))

(event Collision|EventActorBeginOverlap
  (params (OtherActor :type Actor%20Object%20Reference)))

(event EventTick
  (params (DeltaSeconds :type Float%20%28single-precision%29))
  (CallFunction|EnemyStart))

(fn ConstructionScript)

(fn SingleSphereCheck
  (bind _capsulecomponent (Variables|Default|GetCapsuleComponent))
  (bind _returnvalue (Transformation|GetWorldLocation _capsulecomponent))
  (bind (_outhit _returnvalue_2) (Collision|SphereTraceByChannel _returnvalue _returnvalue (Variables|Default|GetDetectionRadius) "TraceTypeQuery3" false 0 "ForOneFrame"))
  (if _returnvalue_2
    (Utilities|Casting|CastToMainCharacter_BP (.HitActor (Collision|BreakHitResult _outhit))
      (:then
        (bind _output_get (Variables|Default|SetChDetected true))
        (return _output_get))
      (:CastFailed
        (bind _output_get_2 (Variables|Default|SetChDetected false))
        (return _output_get_2)))))

(fn CheckVision
  (params (Target :type Main%20Character%20BP%20Object%20Reference))
  (Utilities|IsValid Target
    (:Is%20Valid
      (bind _outhit (Collision|LineTraceByChannel (Transformation|GetWorldLocation (Variables|Default|GetEyes)) (Transformation|GetActorLocation Target) "TraceTypeQuery1" false 0 "ForOneFrame"))
      (Utilities|Casting|CastToMainCharacter_BP (.HitActor (Collision|BreakHitResult _outhit))
        (:then
          (return true))
        (:CastFailed
          (return false))))))

(fn LimitLeft
  (bind _capsulecomponent (Variables|Default|GetCapsuleComponent))
  (bind _capsulecomponent_2 (Variables|Default|GetCapsuleComponent))
  (bind (_origin _boxextent) (Collision|GetComponentBounds _capsulecomponent))
  (bind (_origin_2 _boxextent_2) (Collision|GetComponentBounds _capsulecomponent_2))
  (bind _returnvalue (Collision|LineTraceByChannel (Math|Vector|MakeVector (- (.x _origin_2) (.x _boxextent_2)) (.y _origin_2) (- (.z _origin_2) (.z _boxextent_2))) (Math|Vector|MakeVector (- (.x _origin) (.x _boxextent)) (.y _origin) (- (.z _origin) 1e+02)) "TraceTypeQuery1" false 0 "ForOneFrame"))
  (return _returnvalue))

(fn LimitRight
  (bind _capsulecomponent (Variables|Default|GetCapsuleComponent))
  (bind _capsulecomponent_2 (Variables|Default|GetCapsuleComponent))
  (bind (_origin _boxextent) (Collision|GetComponentBounds _capsulecomponent))
  (bind (_origin_2 _boxextent_2) (Collision|GetComponentBounds _capsulecomponent_2))
  (bind _returnvalue (Collision|LineTraceByChannel (Math|Vector|MakeVector (+ (.x _origin_2) (.x _boxextent_2)) (.y _origin_2) (- (.z _origin_2) (.z _boxextent_2))) (Math|Vector|MakeVector (+ (.x _origin) (.x _boxextent)) (.y _origin) (- (.z _origin) 1e+02)) "TraceTypeQuery1" false 0 "ForOneFrame"))
  (return _returnvalue))

(fn Patrol
  (Utilities|FlowControl|Sequence
    (:then_0
      (bind _detected (CallFunction|LimitRight))
      (if _detected
        _))
    (:then_1
      (bind _detected_2 (CallFunction|LimitLeft))
      (if _detected_2
        _))))

(fn Movement
  (bind _returnvalue (Transformation|GetActorLocation))
  (Transformation|SetActorLocation (Math|Vector|MakeVector (+ (* 0.0 (Variables|Default|Getspeed) (Utilities|Time|GetWorldDeltaSeconds)) (.x _returnvalue)) (.y _returnvalue) (.z _returnvalue)) false false))