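; Archer enemy that senses the player, faces them along the X axis and can fire Arrow_Fatma projectiles from a shooting point.
; Each Tick, a sphere trace sets Attacking and runs an eye line trace whose result is unused; Shoot is not called within this Blueprint.
; DamageEnemy reduces Life, LaunchEnemy applies knockback, and death triggers delayed destruction.
; It updates DDLEGameMode's AmountAlive on spawn and death.
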(event Custom|EnemyCount
  (bind _asddlegame_mode (Utilities|Casting|CastToDDLEGameMode (Game|GetGameMode)))
  (Variables|/Game/FATMA/BluePrints/GameModes/DDLEGameMode.DDLEGameMode_C|SetAmountAlive _asddlegame_mode (- (Variables|/Game/FATMA/BluePrints/GameModes/DDLEGameMode.DDLEGameMode_C|GetAmountAlive _asddlegame_mode) 1)))

(event EventBeginPlay
  (Utilities|FlowControl|Sequence
    (:then_0
      (bind _asmain_character_bp (Utilities|Casting|CastToMainCharacter_BP (Game|GetPlayerCharacter 0)))
      (Variables|Default|SetPlayerRef _asmain_character_bp))
    (:then_1
      (bind _asddlegame_mode (Utilities|Casting|CastToDDLEGameMode (Game|GetGameMode)))
      (Variables|/Game/FATMA/BluePrints/GameModes/DDLEGameMode.DDLEGameMode_C|SetAmountAlive _asddlegame_mode (+ (Variables|/Game/FATMA/BluePrints/GameModes/DDLEGameMode.DDLEGameMode_C|GetAmountAlive _asddlegame_mode) 1)))))

(event Collision|EventActorBeginOverlap
  (params (OtherActor :type Actor%20Object%20Reference)))

(event EventTick
  (params (DeltaSeconds :type Float%20%28single-precision%29))
  (if (Variables|Default|GetIsDead?%20)
    (Utilities|FlowControl|Delay 2.0)
    (Actor|DestroyActor)
    (CallFunction|EnemyCount)
    (else
      (CallFunction|CheckSense)
      (CallFunction|LookatPlayer))))

(event EventDamageEnemy
  (CallFunction|TakeDamage))

(event EventLaunchEnemy
  (Character|LaunchCharacter "700.000000,0.000000,500.000000" true true))

(fn ConstructionScript)

(fn CheckVision
  (params (Target :type Main%20Character%20BP%20Object%20Reference))
  (bind _returnvalue (Transformation|GetActorLocation Target))
  (Utilities|IsValid Target
    (:Is%20Valid
      (bind _outhit (Collision|LineTraceByChannel (Transformation|GetWorldLocation (Variables|Default|GetEyes)) (Math|Vector|MakeVector (.x _returnvalue) (.y _returnvalue) (+ (.z _returnvalue) 1e+01)) "TraceTypeQuery1" false 0 "ForOneFrame"))
      (Utilities|Casting|CastToMainCharacter_BP (.HitActor (Collision|BreakHitResult _outhit))
        (:then
          (return true))
        (:CastFailed
          (return false))))))

(fn CheckSense
  (bind _capsulecomponent (Variables|Default|GetCapsuleComponent))
  (bind _returnvalue (Transformation|GetWorldLocation _capsulecomponent))
  (bind (_outhit _returnvalue_2) (Collision|SphereTraceByChannel _returnvalue _returnvalue 5e+02 "TraceTypeQuery3" false 0 "ForOneFrame"))
  (if _returnvalue_2
    (bind _asmain_character_bp (Utilities|Casting|CastToMainCharacter_BP (.HitActor (Collision|BreakHitResult _outhit)))
      (:then
        (bind _output_get (Variables|Default|SetPlayerRef _asmain_character_bp))
        (Variables|Default|SetAttacking true)
        (CallFunction|CheckVision _output_get))
      (:CastFailed
        (Variables|Default|SetAttacking false)))
    (else
      (Variables|Default|SetAttacking false))))

(fn Shoot
  (bind _returnvalue (Game|SpawnActorfromClass "/Game/FATMA/BluePrints/Enemy/ArcherEnemy/Arrow_Fatma.Arrow_Fatma_C" (Transformation|GetWorldTransform (Variables|Default|GetShootingPoint)) "AlwaysSpawn" 0 0))
  (Utilities|IsValid _returnvalue
    (:Is%20Valid
      (Default|SetDirectionandRotation _returnvalue))))

(fn LookatPlayer
  ;[1 1 1] LookAt Player
  (Math|Float|CompareFloat (- (.x (Transformation|GetActorLocation (Variables|Default|GetPlayerRef))) (.x (Transformation|GetActorLocation))) 0.0
    (:>
      (Variables|Default|SetDirection 1.0)
      (Transformation|SetActorRotation "0, 0, 0"))
    (:<
      (Variables|Default|SetDirection -1.0)
      (Transformation|SetActorRotation "0.000000,180.000000,0.000000"))))

(fn TakeDamage
  (if (<= (- (Variables|Default|GetLife) (Variables|Default|GetDamage)) 0.0)
    (Variables|Default|SetIsDead?%20 true)
    (else
      (Variables|Default|SetLife (- (Variables|Default|GetLife) (Variables|Default|GetDamage))))))