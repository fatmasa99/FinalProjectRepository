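; Player character for a side-scrolling game with sprite animation, handling movement, dash, jump, attack, defend, pausing and death.
; Tick flips control rotation to face the X velocity, while dash raises walk speed and animation play rate.
; Attack and defend send combo messages to the animation instance, whose Locomotion state machine receives airborne, damaged and dead jumps.
; Lethal damage calls Kill, which disables input and collision, mutes music and shows the game-over menu.
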(event Custom|Kill
  (Utilities|FlowControl|Sequence
    (:then_0
      (if (Variables|Default|GetIsDead)
        (Class|BPIStateRequest|JumpStateRequest(Message) (Variables|/Script/PaperZD.PaperZDAnimationComponent|GetAnimInstance (Variables|Default|GetAnimationComponent)) "Dead" "Locomotion")
        (Input|DisableInput 0)
        (Collision|SetCollisionEnabled (Variables|Default|GetCapsuleComponent) "NoCollision")
        (Utilities|FlowControl|Delay 0.5)
        (Game|SetGamePaused true)
        (bind _returnvalue (UserInterface|CreateWidget "/Game/FATMA/Ui/Widgets/InGame/GameOverMenu.GameOverMenu_C"))
        (UserInterface|Viewport|AddtoViewport _returnvalue 0)
        (Variables|/Script/Engine.PlayerController|SetbShowMouseCursor (Game|GetPlayerController 0) true)))
    (:then_1
      (Class|FMODBlueprintStatics|PlayEvent2D "/Game/FMOD/Events/Transition/GameOver.GameOver")
      (Class|FMODBlueprintStatics|BusSetVolume "/Game/FMOD/Buses/Music.Music" 0.0))))

(event EventBeginPlay)

(event Collision|EventActorBeginOverlap
  (params (OtherActor :type Actor%20Object%20Reference)))

(event EventTick
  (params (DeltaSeconds :type Float%20%28single-precision%29))
  (bind _returnvalue (Pawn|GetController))
  (bind _returnvalue_2 (Pawn|GetController))
  (Math|Float|CompareFloat (.X (Math|Vector|BreakVector (Variables|/Script/Engine.MovementComponent|GetVelocity (Pawn|GetMovementComponent)))) 0.0
    (:>
      ;[0 0.4745 1] Look Right
      (Utilities|IsValid _returnvalue_2
        (:Is%20Valid
          (Pawn|SetControlRotation _returnvalue_2 (Math|Rotator|MakeRotator 0.0 0.0 0.0)))))
    (:<
      ;[0 0.4745 1] Look Left
      (Utilities|IsValid _returnvalue
        (:Is%20Valid
          (Pawn|SetControlRotation _returnvalue (Math|Rotator|MakeRotator 0.0 0.0 1.8e+02)))))))

(event EventOnWalkingOffLedge
  (params (PreviousFloorImpactNormal :type Vector%20%28by%20ref%29 :default "0, 0, 0") (PreviousFloorContactNormal :type Vector%20%28by%20ref%29 :default "0, 0, 0") (PreviousLocation :type Vector%20%28by%20ref%29 :default "0, 0, 0") (TimeDelta :type Float%20%28single-precision%29))
  (Class|PaperZDAnimInstance|JumptoNode (Variables|/Script/PaperZD.PaperZDAnimationComponent|GetAnimInstance (Variables|Default|GetAnimationComponent)) "AirBorne" "Locomotion"))

(event EventOnJumped
  (Class|PaperZDAnimInstance|JumptoNode (Variables|/Script/PaperZD.PaperZDAnimationComponent|GetAnimInstance (Variables|Default|GetAnimationComponent)) "AirBorne" "Locomotion"))

(event Input|ActionEvents|InputActionDash
  (params (Key :type Key%20Structure :default "None"))
  (:Pressed
    (Variables|Default|SetRunPlayRate 1.5)
    (Variables|/Script/Engine.CharacterMovementComponent|SetMaxWalkSpeed (Variables|Character|GetCharacterMovement) 1e+03))
  (:Released
    (Variables|Default|SetRunPlayRate 1.0)
    (Variables|/Script/Engine.CharacterMovementComponent|SetMaxWalkSpeed (Variables|Character|GetCharacterMovement) 7e+02)))

(event Input|ActionEvents|InputActionJump
  (params (Key :type Key%20Structure :default "None"))
  (:Pressed
    (Character|Jump)))

(event Input|ActionEvents|InputActionAttack
  (params (Key :type Key%20Structure :default "None"))
  (:Pressed
    (Class|BPICombo|RequestCombo(Message) (Variables|/Script/PaperZD.PaperZDAnimationComponent|GetAnimInstance (Variables|Default|GetAnimationComponent)) "NewEnumerator0")
    (Variables|Default|SetIsAttacking true)))

(event Input|ActionEvents|InputActionDefend
  (params (Key :type Key%20Structure :default "None"))
  (:Pressed
    (Class|BPICombo|RequestCombo(Message) (Variables|/Script/PaperZD.PaperZDAnimationComponent|GetAnimInstance (Variables|Default|GetAnimationComponent)) "NewEnumerator1")
    (Variables|Default|SetIsDefending true)))

(event Input|ActionEvents|InputActionPauseGame
  (params (Key :type Key%20Structure :default "None"))
  (:Pressed
    (bind _returnvalue (UserInterface|CreateWidget "/Game/FATMA/Ui/Widgets/InGame/PauseMenu.PauseMenu_C"))
    (UserInterface|Viewport|AddtoViewport _returnvalue 0)
    (Game|SetGamePaused true)
    (Variables|/Script/Engine.PlayerController|SetbShowMouseCursor (Game|GetPlayerController 0) true)))

(event Input|AxisEvents|InputAxisForward
  (params (AxisValue :type Float%20%28single-precision%29))
  (Pawn|Input|AddMovementInput "1.000000,0.000000,0.000000" AxisValue false))

(fn ConstructionScript)

(fn SpawnDust
  (bind _sprite (Variables|Default|GetSprite))
  (bind _returnvalue (Transformation|GetWorldTransform _sprite))
  (Game|SpawnActorfromClass "/Game/FATMA/BluePrints/Effects/Land_smoke.Land_smoke_C" (Math|Transform|MakeTransform (.location _returnvalue) (.rotation _returnvalue) "1.000000,1.000000,1.000000") "AlwaysSpawn" 0 0))

(fn TakeDamage
  (if (> (- (Variables|Default|GetLife) (Variables|Default|GetDamage)) 0.0)
    (Variables|Default|SetLife (Math|Float|Clamp(Float) (- (Variables|Default|GetLife) (Variables|Default|GetDamage)) 0.0 (Variables|Default|GetMaxLife)))
    (Class|BPIStateRequest|JumpStateRequest(Message) (Variables|/Script/PaperZD.PaperZDAnimationComponent|GetAnimInstance (Variables|Default|GetAnimationComponent)) "Damaged" "Locomotion")
    (else
      (Variables|Default|SetLife 0.0)
      (Variables|Default|SetIsDead true)
      (CallFunction|Kill))))