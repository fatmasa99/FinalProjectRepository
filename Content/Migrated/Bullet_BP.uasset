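; Bullet projectile actor that flies in a straight line along a stored direction and destroys itself when it overlaps any actor.
; Tick moves it by Speed and delta time without sweeping.
; SetDirectionAndRotation computes the direction toward Target and turns the BulletFB component to face it, but is not called within this Blueprint.
; No damage is applied: TakeDamage is empty and Damage is unused.
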(event Collision|EventActorBeginOverlap
  (params (OtherActor :type Actor%20Object%20Reference))
  (Utilities|FlowControl|Sequence
    (:then_1
      (Actor|DestroyActor))))

(event EventTick
  (params (DeltaSeconds :type Float%20%28single-precision%29))
  (CallFunction|BulletMovement DeltaSeconds))

(fn ConstructionScript)

(fn SetDirectionandRotation
  (Variables|Default|Setdirection (Math|Vector|GetUnitDirection(Vector) (Transformation|GetActorLocation) (Transformation|GetActorLocation (Variables|Default|Gettarget))))
  (Transformation|SetRelativeRotation (Variables|Default|GetBullet_FB) (Math|Rotator|FindLookatRotation (Transformation|GetActorLocation) (Transformation|GetActorLocation (Variables|Default|Gettarget))) false false))

(fn BulletMovement
  (params (deltaSeconds :type Float%20%28double-precision%29))
  (Transformation|SetActorLocation (+ (* (* deltaSeconds (Variables|Default|Getspeed)) (Variables|Default|Getdirection)) (Transformation|GetActorLocation)) false false))