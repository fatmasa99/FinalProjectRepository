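; Side-scrolling player character Blueprint using a Paper2D flipbook, with running, sprinting, jumping and a life pool.
; Input drives X-axis movement and jumps, while Sprint swaps MaxWalkSpeed to 1.5 times the speed cached at BeginPlay.
; While alive, Tick picks the jump, idle or run flipbook and mirrors it by X-scaling with the axis value.
; TakeDamage triggers Death at zero life, playing the death flipbook and disabling input and capsule collision.
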(event EventBeginPlay
  (bind _output_get (Variables|Default|Setspeed (Variables|/Script/Engine.CharacterMovementComponent|GetMaxWalkSpeed (Variables|Character|GetCharacterMovement))))
  (Variables|Default|SetspeedSprint (* _output_get 1.5)))

(event EventTick
  (params (DeltaSeconds :type Float%20%28single-precision%29))
  (if (> (Variables|Default|Getlife) 0.0)
    (if (AI|Components|NavMovement|IsFalling (Variables|Character|GetCharacterMovement))
      (Sprite|SetFlipbook (Variables|Default|GetFlipbook) "/Game/Migrated/Jump_FB.Jump_FB")
      (Components|Timeline|SetLooping (Variables|Default|GetFlipbook) false)
      (Audio|Components|Audio|Play (Variables|Default|GetFlipbook))
      (else
        (Components|Timeline|SetLooping (Variables|Default|GetFlipbook) true)
        (Audio|Components|Audio|Play (Variables|Default|GetFlipbook))
        (if (== (Input|AxisValues|GetMoveRight) 0.0)
          (Sprite|SetFlipbook (Variables|Default|GetFlipbook) "/Game/Migrated/Idle_FB.Idle_FB")
          (else
            (Sprite|SetFlipbook (Variables|Default|GetFlipbook) "/Game/Migrated/Run_FB.Run_FB")
            (Transformation|SetRelativeScale3D (Variables|Default|GetFlipbook) (Math|Vector|MakeVector (Input|AxisValues|GetMoveRight) 1.0 1.0))))))))

(event Input|ActionEvents|InputActionJump
  (params (Key :type Key%20Structure))
  (:Pressed
    (Character|Jump)))

(event Input|ActionEvents|InputActionSprint
  (params (Key :type Key%20Structure))
  (:Pressed
    (Variables|/Script/Engine.CharacterMovementComponent|SetMaxWalkSpeed (Variables|Character|GetCharacterMovement) (Variables|Default|GetspeedSprint)))
  (:Released
    (Variables|/Script/Engine.CharacterMovementComponent|SetMaxWalkSpeed (Variables|Character|GetCharacterMovement) (Variables|Default|Getspeed))))

(event Input|AxisEvents|InputAxisMoveRight
  (params (AxisValue :type Float%20%28single-precision%29))
  (Pawn|Input|AddMovementInput "1.000000,0.0,0.0" AxisValue false))

(fn ConstructionScript)

(fn MoveRightF
  (params (InputAxis :type Float%20%28double-precision%29))
  (bind _returnvalue (Transformation|GetActorLocation))
  (if (== InputAxis 0.0)
    (Sprite|SetFlipbook (Variables|Default|GetFlipbook) "/Game/Migrated/Idle_FB.Idle_FB")
    (else
      (Transformation|SetActorLocation (Math|Vector|MakeVector (+ (* InputAxis (Variables|Default|Getspeed) (Utilities|Time|GetWorldDeltaSeconds)) (.x _returnvalue)) (.y _returnvalue) (.z _returnvalue)) false false)
      (Sprite|SetFlipbook (Variables|Default|GetFlipbook) "/Game/Migrated/Run_FB.Run_FB")
      (Transformation|SetRelativeScale3D (Variables|Default|GetFlipbook) (Math|Vector|MakeVector InputAxis 1.0 1.0)))))

(fn TakeDamage
  (params (damage :type Float%20%28double-precision%29))
  (if (> (- (Variables|Default|Getlife) damage) 0.0)
    (Variables|Default|Setlife (- (Variables|Default|Getlife) damage))
    (else
      (Variables|Default|Setlife 0.0)
      (CallFunction|Death))))

(fn Death
  (bind _flipbook (Variables|Default|GetFlipbook))
  (Sprite|SetFlipbook (Variables|Default|GetFlipbook) "/Game/Migrated/Dead_FB.Dead_FB")
  (Components|Timeline|SetLooping _flipbook false)
  (Audio|Components|Audio|Play _flipbook)
  (Input|DisableInput 0)
  (Collision|SetCollisionEnabled (Variables|Collision|GetCapsuleComponent) "NoCollision"))