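; Paper2D robot enemy that patrols along X, flipping direction when downward traces at either capsule edge find no ground.
; Each Tick, a sphere trace plus an eye-level line-of-sight check looks for MainCharacter_BP and stores it as EnemyTarget.
; On detection it stops moving, switches idle and shoot flipbooks, and calls Shoot after a delay.
; Shoot is currently empty, its projectile-spawn logic disconnected; MultiCheckSense is unused.
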(event EventTick
  (params (DeltaSeconds :type Float%20%28single-precision%29))
  (bind _enemytarget (Variables|Default|GetenemyTarget))
  (bind _chdetected (CallFunction|SingleChechkSphere))
  (if _chdetected
    (Utilities|FlowControl|Sequence
      (:then_0
        (Utilities|FlowControl|Delay 1.0)
        (Sprite|SetFlipbook (Variables|Default|GetSprite) "/Game/Migrated/RobotShoot_FB.RobotShoot_FB")
        (Utilities|IsValid _enemytarget
          (:Is%20Valid
            (CallFunction|Shoot _enemytarget))))
      (:then_1
        (Utilities|FlowControl|DoOnce false :!label _label
          (:Completed
            (Sprite|SetFlipbook (Variables|Default|GetSprite) "/Game/Migrated/RobotIdle_FB.RobotIdle_FB")))))
    (else
      (CallFunction|MoveHorizontal)
      (CallFunction|Patroll)
      (goto _label Reset))))

(fn ConstructionScript)

(fn Patroll
  (Utilities|FlowControl|Sequence
    (:then_0
      (bind _detected (CallFunction|LimitRight))
      (if (not _detected)
        (Variables|Default|Setdirection (* (Variables|Default|Getdirection) -1.0))
        (return)))
    (:then_1
      (bind _detected_2 (CallFunction|LimitLeft))
      (if (not _detected_2)
        (Variables|Default|Setdirection (* (Variables|Default|Getdirection) -1.0))
        (return)))))

(fn LimitRight
  (bind _capsulecomponent (Variables|Collision|GetCapsuleComponent))
  (bind _capsulecomponent_2 (Variables|Collision|GetCapsuleComponent))
  (bind (_origin _boxextent) (Collision|GetComponentBounds _capsulecomponent))
  (bind (_origin_2 _boxextent_2) (Collision|GetComponentBounds _capsulecomponent_2))
  (bind _returnvalue (Collision|LineTraceByChannel (Math|Vector|MakeVector (+ (.x _origin) (.x _boxextent)) (.y _origin) (- (.z _origin) (.z _boxextent))) (Math|Vector|MakeVector (+ (.x _origin_2) (.x _boxextent_2)) (.y _origin_2) (Utilities|Operators|Subtract (.z _origin_2) (.z _boxextent_2) 5e+01)) "TraceTypeQuery1" false 0 "ForOneFrame"))
  (return _returnvalue))

(fn LimitLeft
  (bind _capsulecomponent (Variables|Collision|GetCapsuleComponent))
  (bind _capsulecomponent_2 (Variables|Collision|GetCapsuleComponent))
  (bind (_origin _boxextent) (Collision|GetComponentBounds _capsulecomponent))
  (bind (_origin_2 _boxextent_2) (Collision|GetComponentBounds _capsulecomponent_2))
  (bind _returnvalue (Collision|LineTraceByChannel (Math|Vector|MakeVector (- (.x _origin_2) (.x _boxextent_2)) (.y _origin_2) (- (.z _origin_2) (.z _boxextent_2))) (Math|Vector|MakeVector (- (.x _origin) (.x _boxextent)) (.y _origin) (Utilities|Operators|Subtract (.z _origin) (.z _boxextent) 5e+01)) "TraceTypeQuery1" false 0 "ForOneFrame" true "(R=0.000000,G=0.051178,B=1.000000,A=1.000000)" "(R=0.107088,G=1.000000,B=0.000000,A=1.000000)"))
  (return _returnvalue))

(fn MoveHorizontal
  (bind _returnvalue (Transformation|GetActorLocation))
  (bind _direction (Variables|Default|Getdirection))
  (Transformation|SetActorLocation (Math|Vector|MakeVector (+ (* _direction (Variables|Default|Getspeed) (Utilities|Time|GetWorldDeltaSeconds)) (.x _returnvalue)) (.y _returnvalue) (.z _returnvalue)) false false)
  (if (== _direction -1.0)
    (Transformation|SetActorRotation (Math|Rotator|MakeRotator 0.0 0.0 1.8e+02))
    (else
      (Transformation|SetActorRotation (Math|Rotator|MakeRotator 0.0 0.0 0.0)))))

(fn MultiCheckSense
  (bind _capsulecomponent (Variables|Collision|GetCapsuleComponent))
  (bind _returnvalue (Transformation|GetWorldLocation _capsulecomponent))
  (bind _outhits (Collision|MultiSphereTraceByChannel _returnvalue _returnvalue (Variables|Default|GetdetectionRadius) "TraceTypeQuery3" false 0 "ForOneFrame"))
  (for _array_element _outhits
    (Utilities|Casting|CastToMainCharacter_BP (.HitActor (Collision|BreakHitResult _array_element)))
    (return true))
  (return false))

(fn SingleChechkSphere
  (bind _capsulecomponent (Variables|Collision|GetCapsuleComponent))
  (bind _returnvalue (Transformation|GetWorldLocation _capsulecomponent))
  (bind (_outhit _returnvalue_2) (Collision|SphereTraceByChannel _returnvalue _returnvalue (Variables|Default|GetdetectionRadius) "TraceTypeQuery3" false 0 "ForOneFrame"))
  (if _returnvalue_2
    (bind _asmain_character_bp (Utilities|Casting|CastToMainCharacter_BP (.HitActor (Collision|BreakHitResult _outhit))))
    (bind _output_get (Variables|Default|SetenemyTarget _asmain_character_bp))
    (bind _detected (CallFunction|CheckVision _output_get))
    (if _detected
      (return true)
      (else
        (return false)))
    (else
      (Variables|Default|SetenemyTarget 0))))

(fn CheckVision
  (params (target :type Character%20Object%20Reference))
  (Utilities|IsValid target
    (:Is%20Valid
      (bind _outhit (Collision|LineTraceByChannel (Transformation|GetWorldLocation (Variables|Default|GetEyes)) (Transformation|GetActorLocation target) "TraceTypeQuery1" false 0 "ForOneFrame"))
      (Utilities|Casting|CastToMainCharacter_BP (.HitActor (Collision|BreakHitResult _outhit))
        (:then
          (return true))
        (:CastFailed
          (return false))))))

(fn Shoot
  (params (eTarget :type Character%20Object%20Reference)))