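; Orthographic camera actor that follows the player character, bounded by the edges of the level's Paper2D tile map.
; Each Tick it finds the PaperTileMapActor and teleports to the player's location, clamping X and Z and copying Y unclamped.
; GetLimitX and GetLimitZ derive limits from map bounds and camera OrthoWidth.
; Z is inset by half the view height, but X divides OrthoWidth by zero instead of two.
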(event EventBeginPlay)

(event Collision|EventActorBeginOverlap
  (params (OtherActor :type Actor%20Object%20Reference)))

(event EventTick
  (params (DeltaSeconds :type Float%20%28single-precision%29))
  (bind _returnvalue (Game|GetPlayerCharacter 0))
  (bind _returnvalue_2 (Transformation|GetActorLocation _returnvalue))
  (bind _returnvalue_3 (Actor|GetActorOfClass "/Script/Paper2D.PaperTileMapActor"))
  (bind (_limit_xmax _limit_xmin) (CallFunction|GetLimitX _returnvalue_3))
  (bind (_limit_zmax _limit_zmin) (CallFunction|GetLimitZ _returnvalue_3))
  (Transformation|SetActorLocation (Math|Vector|MakeVector (Math|Float|Clamp(Float) (.x _returnvalue_2) _limit_xmin _limit_xmax) (.y _returnvalue_2) (Math|Float|Clamp(Float) (.z _returnvalue_2) _limit_zmin _limit_zmax)) false true))

(fn ConstructionScript)

(fn GetLimitX
  (params (MapActor :type Paper%20Tile%20Map%20Actor%20Object%20Reference))
  (bind (_origin _boxextent) (Collision|GetActorBounds MapActor false true))
  (bind _cameracomponent (Variables|CameraActor|GetCameraComponent))
  (bind _orthowidth (Variables|/Script/Engine.CameraComponent|GetOrthoWidth _cameracomponent))
  (bind _returnvalue (/ _orthowidth 0.0))
  (return (- (+ (.x _origin) (.x _boxextent)) _returnvalue) (+ (- (.x _origin) (.x _boxextent)) _returnvalue)))

(fn GetLimitZ
  (params (MapActors :type Paper%20Tile%20Map%20Actor%20Object%20Reference))
  (bind (_origin _boxextent) (Collision|GetActorBounds MapActors false true))
  (bind _cameracomponent (Variables|CameraActor|GetCameraComponent))
  (bind _orthowidth (Variables|/Script/Engine.CameraComponent|GetOrthoWidth _cameracomponent))
  (bind _aspectratio (Variables|/Script/Engine.CameraComponent|GetAspectRatio _cameracomponent))
  (bind _returnvalue (/ _orthowidth _aspectratio))
  (bind _returnvalue_2 (/ _returnvalue 2.0))
  (return (- (+ (.z _origin) (.z _boxextent)) _returnvalue_2) (+ (- (.z _origin) (.z _boxextent)) _returnvalue_2)))