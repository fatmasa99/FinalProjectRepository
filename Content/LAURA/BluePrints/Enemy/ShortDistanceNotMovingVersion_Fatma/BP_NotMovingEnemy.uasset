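; Stationary enemy character that detects the player and turns to face them along the X axis.
; Each tick while alive, a sphere trace around it looks for MainCharacter_BP, updates the attack flags and snaps its facing.
; Damage drains health until death removes the capsule, then the actor after a delay; LaunchEnemy applies a fixed knock-style launch.
; Patrol movement and ledge-check logic remains but is unused.
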(event Custom|MovementUpdate
  (bind _returnvalue (Transformation|GetActorLocation))
  (bind _detectiondistance (Variables|Default|GetdetectionDistance))
  (if (not (Variables|Default|Getdead))
    (bind (_outhit _returnvalue_2) (Collision|SphereTraceByChannel (+ _returnvalue _detectiondistance) (- _returnvalue _detectiondistance) (Variables|Default|GetRadius) "TraceTypeQuery3" false 0 "ForOneFrame"))
    (if _returnvalue_2
      (bind _asmain_character_bp (Utilities|Casting|CastToMainCharacter_BP (.hitactor _outhit))
        (:then
          (Variables|Default|Setattacking true)
          (Variables|Default|SetplayerRef _asmain_character_bp)
          ;[1 1 1] LookAt Player
          (Math|Float|CompareFloat (- (.x (Transformation|GetActorLocation (Variables|Default|GetplayerRef))) (.x (Transformation|GetActorLocation))) 0.0
            (:>
              ;[1 1 1] Movement
              (Transformation|SetActorRotation "0, 0, 0"))
            (:<
              (Transformation|SetActorRotation "0.000000,180.000000,0.000000"))))
        (:CastFailed
          (Variables|Default|Setattacking false)
          (Variables|Default|Setattacking2 false)))
      (else
        (Variables|Default|Setattacking false)))))

(event EventBeginPlay
  (Utilities|FlowControl|Sequence
    (:then_0
      (Variables|Default|SetmaxEnemyHealth 2e+01)
      (Variables|Default|Setdead false))
    (:then_1
      (bind _asmain_character_bp (Utilities|Casting|CastToMainCharacter_BP (Game|Player|GetPlayerPawn 0)))
      (Variables|Default|SetChaarcterRef _asmain_character_bp))))

(event Collision|EventActorBeginOverlap
  (params (OtherActor :type Actor%20Object%20Reference)))

(event EventLaunchEnemy
  (Character|LaunchCharacter "1000.000000,0.000000,700.000000" true false))

(event Game|Damage|EventAnyDamage
  (params (Damage :type Float%20%28single-precision%29) (DamageType :type Damage%20Type%20Object%20Reference) (InstigatedBy :type Controller%20Object%20Reference) (DamageCauser :type Actor%20Object%20Reference))
  ;[1 1 1] Life Manager
  (bind _output_get (Variables|Default|SetmaxEnemyHealth (- (Variables|Default|GetmaxEnemyHealth) Damage)))
  (if (<= _output_get 0.0)
    (Variables|Default|Setdead true)
    (Components|DestroyComponent (Variables|Default|GetCapsuleComponent))
    (Utilities|FlowControl|Delay 1e+01)
    (Actor|DestroyActor)))

(event EventTick
  (params (DeltaSeconds :type Float%20%28single-precision%29))
  (CallFunction|MovementUpdate))

(fn ConstructionScript)

(fn LimitLeft
  (bind _capsulecomponent (Variables|Default|GetCapsuleComponent))
  (bind _capsulecomponent_2 (Variables|Default|GetCapsuleComponent))
  (bind (_origin _boxextent) (Collision|GetComponentBounds _capsulecomponent))
  (bind (_origin_2 _boxextent_2) (Collision|GetComponentBounds _capsulecomponent_2))
  (bind _returnvalue (Collision|LineTraceByChannel (Math|Vector|MakeVector (+ (.x _origin_2) (.x _boxextent_2)) (.y _origin_2) (- (.z _origin_2) (.z _boxextent_2))) (Math|Vector|MakeVector (+ (.x _origin) (.x _boxextent)) (.y _origin) (- (.z _origin) 5e+02)) "TraceTypeQuery1" false 0 "ForOneFrame"))
  (return _returnvalue))

(fn LimitRight
  (bind _capsulecomponent (Variables|Default|GetCapsuleComponent))
  (bind _capsulecomponent_2 (Variables|Default|GetCapsuleComponent))
  (bind (_origin _boxextent) (Collision|GetComponentBounds _capsulecomponent))
  (bind (_origin_2 _boxextent_2) (Collision|GetComponentBounds _capsulecomponent_2))
  (bind _returnvalue (Collision|LineTraceByChannel (Math|Vector|MakeVector (- (.x _origin_2) (.x _boxextent_2)) (.y _origin_2) (- (.z _origin_2) (.z _boxextent_2))) (Math|Vector|MakeVector (- (.x _origin) (.x _boxextent)) (.y _origin) (- (.z _origin) 5e+02)) "TraceTypeQuery1" false 0 "ForOneFrame"))
  (return _returnvalue))

(fn Patrol
  (Utilities|FlowControl|Sequence
    (:then_0
      (bind _returnvalue (CallFunction|LimitLeft))
      (if (not _returnvalue)
        (Variables|Default|SetmovementDirection (* (Variables|Default|GetmovementDirection) -1.0))))
    (:then_1
      (bind _returnvalue_2 (CallFunction|LimitRight))
      (if (not _returnvalue_2)
        (Variables|Default|SetmovementDirection (* (Variables|Default|GetmovementDirection) -1.0))))))