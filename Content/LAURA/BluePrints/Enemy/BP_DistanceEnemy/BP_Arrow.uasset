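; BP_Arrow is an enemy projectile, fired at the player, that damages MainCharacter_BP on overlap.
; SetDirectionAndRotation stores a unit direction toward PlayerRef's current location and rotates the arrow to face it.
; Tick moves the arrow along that fixed direction at Speed, scaled by delta time and without sweep.
; Overlap applies fixed damage, and the file shows no destruction of the arrow afterwards.
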(event EventBeginPlay)

(event Collision|EventActorBeginOverlap
  (params (OtherActor :type Actor%20Object%20Reference))
  (bind _asmain_character_bp (Utilities|Casting|CastToMainCharacter_BP OtherActor))
  (Game|Damage|ApplyDamage _asmain_character_bp 1e+01 0 0))

(event EventTick
  (params (DeltaSeconds :type Float%20%28single-precision%29))
  (Transformation|SetActorLocation (+ (* (* DeltaSeconds (Variables|Default|Getspeed)) (Variables|Default|Getdirection)) (Transformation|GetActorLocation)) false false))

(fn ConstructionScript)

(fn SetDirectionandRotation
  (Variables|Default|Setdirection (Math|Vector|GetUnitDirection(Vector) (Transformation|GetActorLocation) (Transformation|GetActorLocation (Variables|Default|GetPlayerRef))))
  (Transformation|SetActorRelativeRotation (Math|Rotator|FindLookatRotation (Transformation|GetActorLocation) (Transformation|GetActorLocation (Variables|Default|GetPlayerRef)))))