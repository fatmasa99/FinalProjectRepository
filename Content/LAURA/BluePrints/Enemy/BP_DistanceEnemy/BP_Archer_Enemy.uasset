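; Archer enemy for a side-scrolling layout that patrols along X and stops to face the player when detected.
; Tick runs movement: a forward sphere trace triggers a timed pause and direction flip through a resettable DoOnce.
; A radius trace sets Attacking and PlayerRef, halting patrol; no firing logic exists here.
; Damage drains health; death stops movement updates, removes the capsule and destroys the actor after a delay.
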(event Custom|MovementUpdate
  (bind _returnvalue (Transformation|GetActorLocation))
  (bind _returnvalue_2 (Transformation|GetActorLocation))
  (if (not (Variables|Default|Getdead))
    (Utilities|FlowControl|Sequence
      (:then_0
        ;[1 1 1] Change directions WHEN PATROLLING
        (if (> (Variables|Default|GetmovementDirection) 0.0)
          (Transformation|SetActorRotation "0, 0, 0")
          (else
            (Transformation|SetActorRotation "0.000000,180.000000,0.000000"))))
      (:then_1
        (if (not (Variables|Default|Getattacking))
          ;[1 1 1] Movement
          (Pawn|Input|AddMovementInput "1.000000,0.000000,0.000000" (Variables|Default|GetmovementDirection) false)
          (bind (_outhit _returnvalue_3) (Collision|SphereTraceByChannel _returnvalue_2 (+ _returnvalue_2 (* (Transformation|GetActorForwardVector) (Math|Vector|MakeVector 75.0 0.0 0.0))) 5e+01 "TraceTypeQuery1" false 0 "ForOneFrame"))
          (if _returnvalue_3
            ;;[1 1 1] If something detected
            (Utilities|FlowControl|DoOnce false :!label _label
              (:Completed
                (Variables|/Script/Engine.CharacterMovementComponent|SetMaxWalkSpeed (Variables|Character|GetCharacterMovement) 0.0)
                (Utilities|FlowControl|Delay (Variables|Default|GetDuration))
                (Variables|/Script/Engine.CharacterMovementComponent|SetMaxWalkSpeed (Variables|Character|GetCharacterMovement) (Variables|Default|GetMax%20Walk%20Speed))
                (Variables|Default|SetmovementDirection (* (Variables|Default|GetmovementDirection) -1.0))
                (goto _label Reset))))))
      (:then_2
        (bind (_outhit_2 _returnvalue_4) (Collision|SphereTraceByChannel _returnvalue _returnvalue (Variables|Default|GetdetectionRadius) "TraceTypeQuery3" false 0 "ForOneFrame"))
        (Development|PrintString (Utilities|GetDisplayName (.hitactor _outhit_2)))
        (if _returnvalue_4
          (bind _asmain_character_bp (Utilities|Casting|CastToMainCharacter_BP (.hitactor _outhit_2))
            (:then
              (Variables|Default|Setattacking true)
              (Variables|Default|SetplayerRef _asmain_character_bp)
              (Math|Float|CompareFloat (- (.x (Transformation|GetActorLocation (Variables|Default|GetplayerRef))) (.x (Transformation|GetActorLocation))) 0.0
                (:>
                  (Transformation|SetActorRotation "0, 0, 0"))
                (:<
                  (Transformation|SetActorRotation "0.000000,180.000000,0.000000"))))
            (:CastFailed
              (Variables|Default|Setattacking false)))
          (else
            (Variables|Default|Setattacking false)))))))

(event EventBeginPlay
  (Variables|Default|SetmaxEnemyHealth 2e+01)
  (Variables|Default|Setdead false))

(event Collision|EventActorBeginOverlap
  (params (OtherActor :type Actor%20Object%20Reference)))

(event EventTick
  (params (DeltaSeconds :type Float%20%28single-precision%29))
  (CallFunction|MovementUpdate))

(event Game|Damage|EventAnyDamage
  (params (Damage :type Float%20%28single-precision%29) (DamageType :type Damage%20Type%20Object%20Reference) (InstigatedBy :type Controller%20Object%20Reference) (DamageCauser :type Actor%20Object%20Reference))
  ;[1 1 1] Life Manager
  (bind _output_get (Variables|Default|SetmaxEnemyHealth (- (Variables|Default|GetmaxEnemyHealth) Damage)))
  (if (<= _output_get 0.0)
    (Variables|Default|Setdead true)
    (Components|DestroyComponent (Variables|Default|GetCapsuleComponent))
    (Utilities|FlowControl|Delay 1e+01)
    (Actor|DestroyActor)))

(fn ConstructionScript)