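; BP_ShortDistanceEnemy is a side-scrolling melee enemy that patrols along X and reacts to MainCharacter_BP.
; Tick drives movement: a forward sphere trace pauses and reverses the patrol at obstacles, while a second trace sets Attacking and turns it toward the player.
; DamageEnemy reduces health, then destroys the actor after a delay once dead; LaunchEnemy applies a fixed knockback.
; It increments DDLEGameMode's AmountAlive on BeginPlay and decrements it on death.
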(event Custom|EnemyCount
  (bind _asddlegame_mode (Utilities|Casting|CastToDDLEGameMode (Game|GetGameMode)))
  (Variables|/Game/FATMA/BluePrints/GameModes/DDLEGameMode.DDLEGameMode_C|SetAmountAlive _asddlegame_mode (- (Variables|/Game/FATMA/BluePrints/GameModes/DDLEGameMode.DDLEGameMode_C|GetAmountAlive _asddlegame_mode) 1)))

(event Custom|MovementUpdate
  (bind _returnvalue (Transformation|GetActorLocation))
  (bind _returnvalue_2 (Transformation|GetActorLocation))
  (bind _detectiondistance (Variables|Default|GetdetectionDistance))
  (if (not (Variables|Default|Getdead))
    (Utilities|FlowControl|Sequence
      (:then_0
        ;[1 1 1] Change directions
        (if (> (Variables|Default|GetmovementDirection) 0.0)
          (Transformation|SetActorRotation "0, 0, 0")
          (else
            (Transformation|SetActorRotation "0.000000,180.000000,0.000000"))))
      (:then_1
        ;[1 1 1] Movement
        (if (not (or (Variables|Default|Getattacking) (Variables|Default|Getattacking2)))
          (Pawn|Input|AddMovementInput "1.000000,0.000000,0.000000" (Variables|Default|GetmovementDirection) false)
          (bind (_outhit _returnvalue_3) (Collision|SphereTraceByChannel _returnvalue_2 (+ _returnvalue_2 (* (Transformation|GetActorForwardVector) (Math|Vector|MakeVector 75.0 0.0 0.0))) (Variables|Default|GetRadiusMovement) "TraceTypeQuery1" false 0 "ForOneFrame"))
          (if _returnvalue_3
            ;;[1 1 1] If something detected
            (Utilities|FlowControl|DoOnce false :!label _label
              (:Completed
                (Variables|/Script/Engine.CharacterMovementComponent|SetMaxWalkSpeed (Variables|Character|GetCharacterMovement) 0.0)
                (Utilities|FlowControl|Delay (Variables|Default|GetDuration_0))
                (Variables|/Script/Engine.CharacterMovementComponent|SetMaxWalkSpeed (Variables|Character|GetCharacterMovement) (Variables|Default|GetMax%20Walk%20Speed))
                (Variables|Default|SetmovementDirection (* (Variables|Default|GetmovementDirection) -1.0))
                (goto _label Reset))))))
      (:then_2
        (bind (_outhit_2 _returnvalue_4) (Collision|SphereTraceByChannel (+ _returnvalue _detectiondistance) (- _returnvalue _detectiondistance) (Variables|Default|GetRadius) "TraceTypeQuery3" false 0 "ForOneFrame"))
        (if _returnvalue_4
          (bind _asmain_character_bp (Utilities|Casting|CastToMainCharacter_BP (.hitactor _outhit_2))
            (:then
              (Variables|Default|Setattacking true)
              (Variables|Default|SetplayerRef _asmain_character_bp)
              ;[1 1 1] LookAt Player
              (Math|Float|CompareFloat (- (.x (Transformation|GetActorLocation (Variables|Default|GetplayerRef))) (.x (Transformation|GetActorLocation))) 0.0
                (:>
                  (Transformation|SetActorRotation "0, 0, 0"))
                (:<
                  (Transformation|SetActorRotation "0.000000,180.000000,0.000000"))))
            (:CastFailed
              (Variables|Default|Setattacking false)
              (Variables|Default|Setattacking2 false)))
          (else
            (Variables|Default|Setattacking false)))))))

(event EventBeginPlay
  (Utilities|FlowControl|Sequence
    (:then_0
      (Variables|Default|SetmaxEnemyHealth 2e+01)
      (Variables|Default|Setdead false))
    (:then_1
      (bind _asmain_character_bp (Utilities|Casting|CastToMainCharacter_BP (Game|Player|GetPlayerPawn 0)))
      (Variables|Default|SetChaarcterRef _asmain_character_bp))
    (:then_2
      (bind _asddlegame_mode (Utilities|Casting|CastToDDLEGameMode (Game|GetGameMode)))
      (Variables|/Game/FATMA/BluePrints/GameModes/DDLEGameMode.DDLEGameMode_C|SetAmountAlive _asddlegame_mode (+ (Variables|/Game/FATMA/BluePrints/GameModes/DDLEGameMode.DDLEGameMode_C|GetAmountAlive _asddlegame_mode) 1)))))

(event EventLaunchEnemy
  ;[0.8196 1 0.6745] TakeDamageFromCharacter(Fatma)
  (Character|LaunchCharacter "1000.000000,0.000000,700.000000" true false))

(event Game|Damage|EventAnyDamage
  (params (Damage :type Float%20%28single-precision%29) (DamageType :type Damage%20Type%20Object%20Reference) (InstigatedBy :type Controller%20Object%20Reference) (DamageCauser :type Actor%20Object%20Reference))
  ;[1 1 1] Life Manager
)

(event EventDamageEnemy
  ;[0.8196 1 0.6745] TakeDamageFromCharacter(Fatma)
  (CallFunction|TakeDamage)
  (if (Variables|Default|Getdead)
    (Utilities|FlowControl|Delay 3.0)
    (Actor|DestroyActor)
    (CallFunction|EnemyCount)))

(event EventTick
  (params (DeltaSeconds :type Float%20%28single-precision%29))
  (CallFunction|MovementUpdate))

(fn ConstructionScript)

(fn TakeDamage
  (if (== (- (Variables|Default|GetmaxEnemyHealth) (Variables|Default|GetDamage)) 0.0)
    (Variables|Default|Setdead true)
    (else
      (Variables|Default|SetmaxEnemyHealth (Math|Float|Clamp(Float) (- (Variables|Default|GetmaxEnemyHealth) (Variables|Default|GetDamage)) 0.0 (Variables|Default|GetmaxEnemyHealth))))))